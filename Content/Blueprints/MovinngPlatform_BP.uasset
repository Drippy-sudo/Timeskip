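; Moving platform actor that slides a Platform component between marker points when play begins.
; A timeline, scaled by PlayRate, drives a Lerp of the platform's world location toward EndPoint, without sweep.
; A parallel Sequence branch immediately replaces the captured start location with StartPoint's, then reverses the timeline after a short fixed delay, with no looping in the graph.
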(event `self.ReceiveBeginPlay`
  (`|ExecutionSequence`
    (:`then_0`
      (set `self.StartLocation` (`SceneComponent.K2_GetComponentLocation` (`self.Platform`)))
      (set `self.EndLocation` (`SceneComponent.K2_GetComponentLocation` (`self.End_Point`)))
      (`TimelineComponent.SetPlayRate` (`self.PlatformMove`) (`self.PlayRate`))
      (bind (_direction _newtrack_0) (`Timeline|PlatformMove` :!label _label)
        (:`Update`
          (`SceneComponent.K2_SetWorldLocation` (`self.Platform`) (`KismetMathLibrary.VLerp` (`self.StartLocation`) (`self.EndLocation`) _newtrack_0) false false))))
    (:`then_1`
      (set `self.StartLocation` (`SceneComponent.K2_GetComponentLocation` (`self.Start_Point`)))
      (`KismetSystemLibrary.Delay` 1.0)
      (goto _label :!via `Reverse`))))

(fn `UserConstructionScript`)