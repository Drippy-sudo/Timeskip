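; Charger enemy AI actor that takes sword damage from the player and is destroyed when its health runs out.
; Capsule overlaps with a sword actor count as hits only while the first player character's outward-slash flag is set.
; Each hit prints a debug string and subtracts a fixed amount of health.
; No movement or charge behavior is scripted in these graphs.
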(event `self.CapsuleComponent.OnComponentBeginOverlap`
  (params (OverlappedComponent :type "PrimitiveComponent Object Reference") (OtherActor :type "Actor Object Reference") (OtherComp :type "PrimitiveComponent Object Reference") (OtherBodyIndex :type Integer) (bFromSweep :type Boolean) (SweepResult :type "HitResult Structure (by ref)"))
  (cast `/Game/Character/Weapons/Blueprints/Weapon_Sword` OtherActor)
  (bind _asbp_character (cast `/Game/BP_Character` (`GameplayStatics.GetPlayerCharacter` 0)))
  (if (`/Game/BP_Character.SlashSword Outwards` _asbp_character)
    (`KismetSystemLibrary.PrintString` "Hit")
    (bind _output_get (set `self.Health` (- (`self.Health`) 0.25)))
    (if (<= _output_get 0.0)
      (`self.K2_DestroyActor`))))

(fn `UserConstructionScript`
  (`parent.UserConstructionScript`))