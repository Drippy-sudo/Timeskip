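; Enemy AI pawn that patrols between two locations and chases BP_Character when PawnSensing sees it.
; Each sighting sets the chase flags and moves toward the player, while a retriggerable delay clears visibility once sightings stop.
; Tick ends the chase after a short delayed visibility check and uses a DoOnce gate to start patrol when not chasing.
; Patrol chains AIMoveTo calls in a loop, advancing on success or failure.
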(event `self.PawnSensing.OnSeePawn`
  (params (Pawn :type "Pawn Object Reference"))
  ;[1 1 1] Chase player when seen
  (bind _asbp_character (cast `/Game/BP_Character` Pawn))
  (`|ExecutionSequence`
    (:`then_0`
      (set `self.Can See Enemy?` true)
      (set `self.IsChasing?` true)
      (`|AIMoveTo` self (0.0 0.0 0.0) _asbp_character
        (:`then`
          (`/Engine/EditorBlueprintResources/StandardMacros.DoOnce` false :!label _label))))
    (:`then_1`
      (`KismetSystemLibrary.RetriggerableDelay` 1.0)
      (set `self.Can See Enemy?` false))))

(event `self.ReceiveTick`
  (params (DeltaSeconds :type "Float (single-precision)"))
  (`|ExecutionSequence`
    (:`then_0`
      ;[1 1 1] Chase player when seen
      (if (`self.Can See Enemy?`)
        (`KismetSystemLibrary.Delay` 0.4)
        (if (not (`self.Can See Enemy?`))
          (set `self.IsChasing?` false)
          (goto _label :!via `Reset`))))
    (:`then_1`
      ;[1 1 1] Patrolling location
      (if (`self.IsChasing?`)
        (goto _label_2 :!via `Reset`)
        (else
          (`/Engine/EditorBlueprintResources/StandardMacros.DoOnce` false :!label _label_2
            (:`Completed`
              (`|AIMoveTo` self (`self.Location 1`) null :!label _label_3
                (:`OnSuccess`
                  _)
                (:`OnFail`
                  _))
              (`|AIMoveTo` self (`self.Location 2`) null
                (:`OnSuccess`
                  _)
                (:`OnFail`
                  _))
              (`|ExecutionSequence`
                (:`then_0`
                  (goto _label_3))
                (:`then_1`
                  (goto _label_2 :!via `Reset`))))))))))

(fn `UserConstructionScript`)