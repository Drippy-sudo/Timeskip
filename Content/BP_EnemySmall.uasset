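; BP_EnemySmall is a Blueprint that, despite its enemy name, handles a mouse-following crosshair and a player-input sword attack.
; BeginPlay creates the WBP_Crosshair widget and adds it to the viewport, and Tick moves it to the mouse position.
; The SwordAttack input sets SlashSwordOutwards, which blocks repeat presses until a short delay clears it and prints a debug string.
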(event `self.ReceiveBeginPlay`
  (bind _returnvalue (`|CreateWidget` "/Game/WBP_Crosshair.WBP_Crosshair_C"))
  (bind _output_get (set `self.Crosshair_Widget` _returnvalue))
  (`UserWidget.AddToViewport` _output_get 0))

(event `self.ReceiveTick`
  (params (DeltaSeconds :type "Float (single-precision)"))
  (bind _returnvalue (`WidgetLayoutLibrary.GetMousePositionOnViewport`))
  (`UserWidget.SetPositionInViewport` (`self.Crosshair_Widget`) _returnvalue true))

(event `InputAction|SwordAttack`
  (params (Key :type "Key Structure"))
  ;[1 1 1] Sword Attack
  (:`Pressed`
    (if (not (`self.SlashSword Outwards`))
      (set `self.SlashSword Outwards` true)
      (`KismetSystemLibrary.Delay` 1.0)
      (set `self.SlashSword Outwards` false)
      (`KismetSystemLibrary.PrintString` "Sword"))))

(fn `UserConstructionScript`)